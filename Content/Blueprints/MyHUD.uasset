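; A HUD Blueprint that shows the player's race status for the buggy racing game.
; On BeginPlay it casts player pawn 0 to New_Buggy_BP and stores it.
; Each DrawHUD call draws red text from that pawn: the lap count at top left and the floored race position at top right, offset from the screen width.
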(event `self.ReceiveBeginPlay`
  (bind _asnew_buggy_bp (cast `/Game/The_New_Buggy/New_Buggy_BP` (`GameplayStatics.GetPlayerPawn` 0)))
  (set `self.BuggyPawn` _asnew_buggy_bp))

(event `self.ReceiveDrawHUD`
  (params (SizeX :type Integer) (SizeY :type Integer))
  (bind _buggypawn (`self.BuggyPawn`))
  (set `self.ScreenDimensions` (`KismetMathLibrary.MakeVector2D` (`KismetMathLibrary.Conv_IntToDouble` SizeX) (`KismetMathLibrary.Conv_IntToDouble` SizeY)))
  (`self.DrawText` (`KismetTextLibrary.Conv_TextToString` (`|FormatText` "Lap: {A}" (`KismetTextLibrary.Conv_IntToText` (`/Game/The_New_Buggy/New_Buggy_BP.LapCount` _buggypawn)))) (struct :`R` 1.0 :`A` 1.0) 50.0 50.0 "/Engine/EngineFonts/RobotoDistanceField.RobotoDistanceField" 3.0)
  (`self.DrawText` (`KismetTextLibrary.Conv_TextToString` (`|FormatText` "Pos: {A}" (`KismetTextLibrary.Conv_IntToText` (`KismetMathLibrary.FFloor` (`/Game/The_New_Buggy/New_Buggy_BP.RacePosition` _buggypawn))))) (struct :`R` 1.0 :`A` 1.0) (`KismetMathLibrary.Conv_IntToDouble` (- SizeX 230)) 50.0 "/Engine/EngineFonts/RobotoDistanceField.RobotoDistanceField" 3.0))

(fn `UserConstructionScript`)